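; Moving obstacle that slides between its starting position and an EndLocation, passing overlaps to its parent class for damage.
; On BeginPlay it caches the root's world location, starts MoveLeft, then starts MoveRight three seconds later.
; Each move uses its own timeline to lerp the root's location without sweep, in opposite directions.
; The event graph triggers this out-and-back sequence only once.
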(event `self.ReceiveBeginPlay`
  (set `self.StartLocation` (`SceneComponent.K2_GetComponentLocation` (`self.DefaultSceneRoot`)))
  (`self.Move Left`)
  (`KismetSystemLibrary.Delay` 3.0)
  (`self.Move Right`))

(event `Move Left`
  (bind (_direction _newtrack_0) (`Timeline|Timeline` :!via `PlayFromStart`)
    (:`Update`
      (`SceneComponent.K2_SetWorldLocation` (`self.DefaultSceneRoot`) (`KismetMathLibrary.VLerp` (`self.StartLocation`) (`self.EndLocation`) _newtrack_0) false false))))

(event `Move Right`
  (bind (_direction _newtrack_0) (`Timeline|Timeline_0` :!via `PlayFromStart`)
    (:`Update`
      (`SceneComponent.K2_SetWorldLocation` (`self.DefaultSceneRoot`) (`KismetMathLibrary.VLerp` (`self.EndLocation`) (`self.StartLocation`) _newtrack_0) false false))))

(event `self.ReceiveActorBeginOverlap`
  (params (OtherActor :type "Actor Object Reference"))
  ;[1 1 1] Parent Damage
  (`parent.ReceiveActorBeginOverlap` OtherActor))

(fn `UserConstructionScript`
  (`parent.UserConstructionScript`))