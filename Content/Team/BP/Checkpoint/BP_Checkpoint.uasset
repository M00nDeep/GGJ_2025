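; BP_Checkpoint is a checkpoint actor that saves its own location as the player's position when a Player-tagged actor overlaps its CheckpointBox.
; It writes PlayerPos to a SaveGameObj in slot "1", either loading the existing save or creating a new one.
; The existence check queries an empty slot name rather than "1", so it does not test the slot that is loaded and saved.
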(event `self.CheckpointBox.OnComponentBeginOverlap`
  (params (OverlappedComponent :type "PrimitiveComponent Object Reference") (OtherActor :type "Actor Object Reference") (OtherComp :type "PrimitiveComponent Object Reference") (OtherBodyIndex :type Integer) (bFromSweep :type Boolean) (SweepResult :type "HitResult Structure (by ref)"))
  (bind _returnvalue (`self.K2_GetActorLocation`))
  (if (`self.ActorHasTag` OtherActor "Player")
    (bind _returnvalue_2 (`GameplayStatics.DoesSaveGameExist` ""))
    (if _returnvalue_2
      (bind _returnvalue_3 (`GameplayStatics.LoadGameFromSlot` "1"))
      (bind _assave_game_obj (cast `/Game/Team/BP/Checkpoint/SaveGameObj` _returnvalue_3))
      (set `/Game/Team/BP/Checkpoint/SaveGameObj.PlayerPos` _returnvalue _assave_game_obj)
      (`GameplayStatics.SaveGameToSlot` _assave_game_obj "1")
      (else
        (bind _returnvalue_4 (`GameplayStatics.CreateSaveGameObject` "/Game/Team/BP/Checkpoint/SaveGameObj.SaveGameObj_C"))
        (set `/Game/Team/BP/Checkpoint/SaveGameObj.PlayerPos` _returnvalue _returnvalue_4)
        (`GameplayStatics.SaveGameToSlot` _returnvalue_4 "1")))))

(fn `UserConstructionScript`)