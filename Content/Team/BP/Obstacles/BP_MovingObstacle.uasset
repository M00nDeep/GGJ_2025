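; BP_MovingObstacle is a moving obstacle that defers its overlap handling, noted as damage, to its parent class.
; On BeginPlay it stores the root's relative location, then starts two timelines together.
; Both timelines set the root's world location, lerping between that start and EndLocation in opposite directions.
; Tile-count movement loops and physics-force nudges remain as disconnected, unused logic.
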(event `self.ReceiveBeginPlay`
  (set `self.StartLocation` (`SceneComponent.RelativeLocation` (`self.DefaultSceneRoot`)))
  (`self.LeftMovement`)
  (`self.RightMovement`))

(event `self.ReceiveActorBeginOverlap`
  (params (OtherActor :type "Actor Object Reference"))
  ;[1 1 1] Parent Damage
  (`parent.ReceiveActorBeginOverlap` null))

(event `LeftMovement`
  (bind (_direction _newtrack_0) (`Timeline|Move` :!via `PlayFromStart`)
    (:`Update`
      (`SceneComponent.K2_SetWorldLocation` (`self.DefaultSceneRoot`) (`KismetMathLibrary.VLerp` (`self.StartLocation`) (`self.EndLocation`) _newtrack_0) false false))))

(event `RightMovement`
  (bind (_direction _newtrack_0) (`Timeline|Timeline` :!via `PlayFromStart`)
    (:`Update`
      (`SceneComponent.K2_SetWorldLocation` (`self.DefaultSceneRoot`) (`KismetMathLibrary.VLerp` (`self.EndLocation`) (`self.StartLocation`) _newtrack_0) false false))))

(fn `UserConstructionScript`
  (`parent.UserConstructionScript`))