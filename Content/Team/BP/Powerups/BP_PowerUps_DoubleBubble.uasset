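; Double Bubble powerup that reacts when a Player-tagged actor overlaps its box and sends the character a second-HP message.
; The character's CanBump check decides between pickup and miss, each with its own sound, Niagara burst and camera shake.
; A successful pickup shows a temporary in-game text widget on first encounter, otherwise only on an occasional random roll.
; The asset's own CanBump function just returns false.
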(event `self.Box.OnComponentBeginOverlap`
  (params (OverlappedComponent :type "PrimitiveComponent Object Reference") (OtherActor :type "Actor Object Reference") (OtherComp :type "PrimitiveComponent Object Reference") (OtherBodyIndex :type Integer) (bFromSweep :type Boolean) (SweepResult :type "HitResult Structure (by ref)"))
  (if (`self.ActorHasTag` OtherActor "Player")
    (bind _powerup_ (`/Game/Team/BP/Character/BP_Character.CanBump?` (`self.Character`)))
    (if _powerup_
      (`GameplayStatics.PlaySound2D` null 1.0 1.0 0.0 null null)
      (`NiagaraFunctionLibrary.SpawnSystemAtLocation` "/Niagara/DefaultAssets/Templates/Systems/AttributeReaderTrails.AttributeReaderTrails" (`SceneComponent.K2_GetComponentLocation` (`self.DefaultSceneRoot`)) (struct) (20.0 20.0 20.0))
      (`GameplayStatics.PlayWorldCameraShake` "/Game/Team/BP/CameraShake/CS_TakePowerup.CS_TakePowerup_C" (`SceneComponent.K2_GetComponentLocation` (`/Game/Team/BP/Character/BP_Character.Camera` (`self.Character`))) 50.0 75.0)
      (message `/Game/Team/BP/Interfacce/BPI_PlayerUtility.I_SendSecondHP` (`self.Character`))
      (if (`self.FirstEncounter?`)
        (bind _returnvalue (`|CreateWidget` "/Game/Team/BP/WB/Text/WB_InGameText.WB_InGameText_C" :!label _label))
        (`UserWidget.AddToViewport` _returnvalue 0)
        (`KismetSystemLibrary.Delay` 4.0)
        (`Widget.RemoveFromParent` _returnvalue)
        (elif (>= (`KismetMathLibrary.RandomIntegerInRange` 0 100) 75)
          (goto _label)))
      (else
        (`GameplayStatics.PlaySound2D` null 1.0 1.0 0.0 null null)
        (`NiagaraFunctionLibrary.SpawnSystemAtLocation` "/Niagara/DefaultAssets/Templates/Systems/DirectionalBurst.DirectionalBurst" (`SceneComponent.K2_GetComponentLocation` (`self.DefaultSceneRoot`)) (struct) (20.0 20.0 20.0))
        (`GameplayStatics.PlayWorldCameraShake` "/Game/Team/BP/CameraShake/CS_MissPowerup.CS_MissPowerup_C" (`SceneComponent.K2_GetComponentLocation` (`/Game/Team/BP/Character/BP_Character.Camera` (`self.Character`))) 50.0 75.0)))))

(fn `CanBump?`
  (returns (`Powerup?` :type Boolean))
  (return false))

(fn `UserConstructionScript`)