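; Powerup actor with a box trigger that aims to change a character's speed on overlap.
; On box overlap it calls CanBump on a Character reference and, if true, calls that character's SpeedControl with a fixed value.
; Both branches print a debug string.
; The actor's own SpeedControl and CanBump functions are stubs, returning zero and passing the input through.
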(event `self.Box.OnComponentBeginOverlap`
  (params (OverlappedComponent :type "PrimitiveComponent Object Reference") (OtherActor :type "Actor Object Reference") (OtherComp :type "PrimitiveComponent Object Reference") (OtherBodyIndex :type Integer) (bFromSweep :type Boolean) (SweepResult :type "HitResult Structure (by ref)"))
  (bind _powerup_ (`/Game/Team/BP/Character/BP_Character.CanBump?` (`self.Character`)))
  (if _powerup_
    (`KismetSystemLibrary.PrintString` "true")
    (`/Game/Team/BP/Character/BP_Character.SpeedControl` (`self.Character`) 500.0)
    (else
      (`KismetSystemLibrary.PrintString` "false"))))

(fn `CanBump?`
  (params (`Bump?` :type Boolean :default false))
  (returns (`Powerup?` :type Boolean))
  (return `Bump?`))

(fn `SpeedControl`
  (params (MaxSpeed :type "Float (double-precision)" :default 0.0))
  (returns (NewSpeed :type "Float (double-precision)"))
  (return 0.0))

(fn `UserConstructionScript`)