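; Moving obstacle that slides between lane positions and damages the player on contact.
; A looping timer starts at BeginPlay and runs either a two-lane round trip or, when Trilane is set, a four-leg round trip through MidLocation.
; Each leg is a timeline lerping the root's world location without sweep, with legs spaced by MovementDelay.
; Box overlap with a Player-tagged actor sends a damage interface message to player pawn 0.
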(event `self.Box.OnComponentBeginOverlap`
  (params (OverlappedComponent :type "PrimitiveComponent Object Reference") (OtherActor :type "Actor Object Reference") (OtherComp :type "PrimitiveComponent Object Reference") (OtherBodyIndex :type Integer) (bFromSweep :type Boolean) (SweepResult :type "HitResult Structure (by ref)"))
  ;[1 1 1] Damage
  (if (`self.ActorHasTag` OtherActor "Player")
    (message `/Game/Team/BP/Interfacce/BPI_PlayerUtility.I_SendDamage` (`GameplayStatics.GetPlayerPawn` 0))))

(event `self.ReceiveBeginPlay`
  ;[1 1 1] BeginPlay
  (set `self.StartingLocation` (`SceneComponent.K2_GetComponentLocation` (`self.DefaultSceneRoot`)))
  (`self.StartMovement`))

(event `TriMove`
  ;[1 1 1] TriMove
  (bind (_direction _newtrack_0) (`Timeline|Timeline_1` :!via `PlayFromStart`)
    (:`Update`
      (`SceneComponent.K2_SetWorldLocation` (`self.DefaultSceneRoot`) (`KismetMathLibrary.VLerp` (`self.StartingLocation`) (`self.MidLocation`) _newtrack_0) false false))))

(event `Move`
  ;[1 1 1] Bilane Movement
  (bind (_direction _newtrack_0) (`Timeline|Timeline` :!via `PlayFromStart`)
    (:`Update`
      (`SceneComponent.K2_SetWorldLocation` (`self.DefaultSceneRoot`) (`KismetMathLibrary.VLerp` (`self.StartingLocation`) (`self.EndLocation`) _newtrack_0) false false))))

(event `TriMidMovement`
  ;[1 1 1] TriMove
  (bind (_direction _newtrack_0) (`Timeline|Timeline_3` :!via `PlayFromStart`)
    (:`Update`
      (`SceneComponent.K2_SetWorldLocation` (`self.DefaultSceneRoot`) (`KismetMathLibrary.VLerp` (`self.MidLocation`) (`self.EndLocation`) _newtrack_0) false false))))

(event `ResetMovement`
  ;[1 1 1] Bilane Movement
  (bind (_direction _newtrack_0) (`Timeline|Timeline_0` :!via `PlayFromStart`)
    (:`Update`
      (`SceneComponent.K2_SetWorldLocation` (`self.DefaultSceneRoot`) (`KismetMathLibrary.VLerp` (`self.EndLocation`) (`self.StartingLocation`) _newtrack_0) false false))))

(event `TriResetMove`
  ;[1 1 1] TriMove
  (bind (_direction _newtrack_0) (`Timeline|Timeline_2` :!via `PlayFromStart`)
    (:`Update`
      (`SceneComponent.K2_SetWorldLocation` (`self.DefaultSceneRoot`) (`KismetMathLibrary.VLerp` (`self.EndLocation`) (`self.MidLocation`) _newtrack_0) false false))))

(event `TriFinalMove`
  ;[1 1 1] TriMove
  (bind (_direction _newtrack_0) (`Timeline|Timeline_4` :!via `PlayFromStart`)
    (:`Update`
      (`SceneComponent.K2_SetWorldLocation` (`self.DefaultSceneRoot`) (`KismetMathLibrary.VLerp` (`self.MidLocation`) (`self.StartingLocation`) _newtrack_0) false false))))

(event `StartMovement`
  (`KismetSystemLibrary.K2_SetTimerDelegate` (delegate `LaneMovement`) 4.0 true false 2.0))

(event `LaneMovement`
  (if (`self.Trilane?`)
    (`self.TriMove`)
    (`KismetSystemLibrary.Delay` (`self.MovementDelay`))
    (`self.TriMidMovement`)
    (`KismetSystemLibrary.Delay` (`self.MovementDelay`))
    (`self.TriResetMove`)
    (`KismetSystemLibrary.Delay` (`self.MovementDelay`))
    (`self.TriFinalMove`)
    (else
      (`self.Move`)
      (`KismetSystemLibrary.Delay` (`self.MovementDelay`))
      (`self.ResetMovement`))))

(fn `UserConstructionScript`)