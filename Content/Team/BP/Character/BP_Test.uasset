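; BP_Test is a test character Blueprint with sideways rolls, jump and a timed hover, driven by Enhanced Input.
; Rolls launch the character along world Y while not jumping, with paired left/right counters capping travel each way.
; Jump sets IsJumping behind a DoOnce with no reset, enabling hover, which switches to Flying then back to Walking after a delay.
; Releasing jump or hover shares one path that stops jumping and clears the flag after a delay.
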(event `self.ReceiveBeginPlay`
  (bind _returnvalue (pcsubsystem `EnhancedInputLocalPlayerSubsystem` (`GameplayStatics.GetPlayerController` 0)))
  (`/Engine/EditorBlueprintResources/StandardMacros.IsValid` _returnvalue
    (:`Is Valid`
      (message `EnhancedInputSubsystemInterface.AddMappingContext` _returnvalue "/Game/Team/BP/Character/Input/InputMapping/IM_InGame.IM_InGame" 0 (struct)))))

(event `EnhancedInput|/Game/Team/BP/Character/Input/InputAction/IA_RollLeft`
  (params (ActionValue :type Boolean) (ElapsedSeconds :type "Float (double-precision)") (TriggeredSeconds :type "Float (double-precision)") (InputAction :type "InputAction Object Reference" :default "/Game/Team/BP/Character/Input/InputAction/IA_RollLeft.IA_RollLeft"))
  (:`Completed`
    (if (`self.IsJumping?`)
      _
      (elif (not (== (`self.LeftCount`) (`self.LeftMaxCount`)))
        (`self.LaunchCharacter` (0.0 -2500.0 100.0))
        (set `self.LeftCount` (+ (`self.LeftCount`) 1))
        (set `self.RightCount` (- (`self.RightCount`) 1))))))

(event `EnhancedInput|/Game/Team/BP/Character/Input/InputAction/IA_RollRight`
  (params (ActionValue :type Boolean) (ElapsedSeconds :type "Float (double-precision)") (TriggeredSeconds :type "Float (double-precision)") (InputAction :type "InputAction Object Reference" :default "/Game/Team/BP/Character/Input/InputAction/IA_RollRight.IA_RollRight"))
  (:`Completed`
    (if (`self.IsJumping?`)
      _
      (elif (not (== (`self.RightCount`) (`self.RightMaxCount`)))
        (`self.LaunchCharacter` (0.0 2500.0 100.0))
        (set `self.RightCount` (+ (`self.RightCount`) 1))
        (set `self.LeftCount` (- (`self.LeftCount`) 1))))))

(event `EnhancedInput|/Game/Team/BP/Character/Input/InputAction/IA_Jump`
  (params (ActionValue :type Boolean) (ElapsedSeconds :type "Float (double-precision)") (TriggeredSeconds :type "Float (double-precision)") (InputAction :type "InputAction Object Reference" :default "/Game/Team/BP/Character/Input/InputAction/IA_Jump.IA_Jump"))
  (:`Triggered`
    (`/Engine/EditorBlueprintResources/StandardMacros.DoOnce` false
      (:`Completed`
        (`self.Jump`)
        (set `self.IsJumping?` true)
        (`KismetSystemLibrary.PrintString` "Jump"))))
  (:`Completed`
    (`self.StopJumping` :!label _label)
    (`KismetSystemLibrary.Delay` 0.6)
    (set `self.IsJumping?` false)
    (`KismetSystemLibrary.PrintString` "StopJumping")))

(event `EnhancedInput|/Game/Team/BP/Character/Input/InputAction/IA_Hover`
  (params (ActionValue :type Boolean) (ElapsedSeconds :type "Float (double-precision)") (TriggeredSeconds :type "Float (double-precision)") (InputAction :type "InputAction Object Reference" :default "/Game/Team/BP/Character/Input/InputAction/IA_Hover.IA_Hover"))
  (bind _charactermovement (`self.CharacterMovement`))
  (:`Triggered`
    (if (`self.IsJumping?`)
      (`CharacterMovementComponent.SetMovementMode` _charactermovement "MOVE_Flying" 0)
      (`KismetSystemLibrary.PrintText` "Hower")
      (`KismetSystemLibrary.Delay` 3.0)
      (`CharacterMovementComponent.SetMovementMode` _charactermovement "MOVE_Walking" 0)))
  (:`Completed`
    (goto _label)))

(fn `UserConstructionScript`)