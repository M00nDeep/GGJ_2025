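; BP_PlaySequence is a trigger volume actor that plays an assigned Level Sequence when the player enters it.
; A box overlap with an actor tagged Player creates a sequence player and starts playback.
; When EndSequence is set, it waits SequenceDuration, opens the main menu level and deletes the save in slot "1", acting as a game ending.
; Nothing guards against repeat overlaps retriggering it.
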(event `self.Box.OnComponentBeginOverlap`
  (params (OverlappedComponent :type "PrimitiveComponent Object Reference") (OtherActor :type "Actor Object Reference") (OtherComp :type "PrimitiveComponent Object Reference") (OtherBodyIndex :type Integer) (bFromSweep :type Boolean) (SweepResult :type "HitResult Structure (by ref)"))
  (if (`self.ActorHasTag` OtherActor "Player")
    (bind (_outactor _returnvalue) (`LevelSequencePlayer.CreateLevelSequencePlayer` (`self.Level Sequence`)))
    (`MovieSceneSequencePlayer.Play` _returnvalue)
    (if (`self.EndSequence?`)
      (`KismetSystemLibrary.Delay` (`self.SequenceDuration`))
      (`GameplayStatics.OpenLevelBySoftObjectPtr` "/Game/Team/Maps/MP_MainMenu.MP_MainMenu")
      (`GameplayStatics.DeleteGameInSlot` "1"))))

(fn `UserConstructionScript`)